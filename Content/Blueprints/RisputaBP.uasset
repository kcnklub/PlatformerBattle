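; RisputaBP is a Paper2D character Blueprint that drives Risputa's flipbook animation and death collision.
; Each Tick picks a flipbook through a priority-based state function: dead, attacking, falling, then idle, with the dead state showing RunningAnimation.
; Tick also toggles capsule collision from IsDead and reassigns the Attacking event, whose handler holds the attack state for half a second.
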(event Custom|UpdateAnimation
  ;[1 0 0.1344] Animation State Machine Custom Event
  (bind _output_flipbook (CallFunction|AnimationStateMachine (Variables|Default|GetCurrAttacking) (Variables|Default|GetbIsDead) (AI|Components|NavMovement|IsFalling (Variables|Character|GetCharacterMovement))))
  (Sprite|SetFlipbook (Variables|Default|GetSprite) _output_flipbook))

(event Custom|Attacking_Event_0
  (params (bIsAttacking :type Boolean))
  (Variables|Default|SetCurrAttacking true)
  (Utilities|FlowControl|Delay 0.5)
  (Variables|Default|SetCurrAttacking false))

(event EventTick
  (params (DeltaSeconds :type Float%20%28single-precision%29))
  (Utilities|FlowControl|Sequence
    (:then_0
      (CallFunction|UpdateAnimation))
    (:then_1
      (CallFunction|TurnCollisionOffwhenDead))
    (:then_2
      (EventDispatchers|AssignAttacking (delegate Custom|Attacking_Event_0)))))

(fn ConstructionScript)

(fn AnimationStateMachine
  (params (IsBasicAttack :type Boolean) (IsDead :type Boolean) (IsFalling :type Boolean))
  (LocalVariables|SetIsBasicAttack_Local IsBasicAttack)
  (LocalVariables|SetIsDead_Local IsDead)
  (LocalVariables|SetIsFalling_Local IsFalling)
  (if (LocalVariables|GetIsDead_Local)
    (LocalVariables|SetAnimationState "NewEnumerator2")
    (elif (LocalVariables|GetIsBasicAttack_Local)
      (LocalVariables|SetAnimationState "NewEnumerator1")
      (elif (LocalVariables|GetIsFalling_Local)
        (LocalVariables|SetAnimationState "NewEnumerator3")
        (else
          (LocalVariables|SetAnimationState "NewEnumerator0")))))
  (return (Utilities|Select :Index (LocalVariables|GetAnimationState) :NewEnumerator0 "/Game/FlipBooks/Risputa/idle.idle" :NewEnumerator1 "/Game/FlipBooks/Risputa/AttackAnim.AttackAnim" :NewEnumerator2 "/Game/2dSideScroller/Sprites/RunningAnimation.RunningAnimation" :NewEnumerator3 "/Game/FlipBooks/Dash_SwordMan/Jumping.Jumping")))

(fn TurnCollisionOffwhenDead
  (if (Variables|Default|GetbIsDead)
    (Collision|SetCollisionEnabled (Variables|Default|GetCapsuleComponent) "NoCollision")
    (else
      (Collision|SetCollisionEnabled (Variables|Default|GetCapsuleComponent) "QueryAndPhysics"))))