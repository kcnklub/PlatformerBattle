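; Paper2D dash swordsman character that drives its flipbook animation from movement, landing, death and three attack states.
; Each Tick it updates the sprite, turns capsule collision off while dead and re-binds the three attack dispatchers, whose handlers set timed flags.
; A nested-branch state function prioritizes attacks, then landing, death, falling and running over idle, with several states sharing or borrowing flipbooks.
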(event Custom|SecondAttack_Event_0
  (params (HasAttackedTwice :type Boolean))
  (Variables|Default|SetHasAttackTwice true)
  (Utilities|FlowControl|Delay 0.5)
  (Variables|Default|SetHasAttackTwice false))

(event Custom|UpdateAnimation
  (bind _output_flipbook (CallFunction|AnimationStateMachine (AI|Components|NavMovement|IsFalling (Variables|Character|GetCharacterMovement)) (> (Math|Vector|VectorLength (Transformation|GetVelocity)) 0.0) (Variables|Default|GetbIsDead) (Variables|Default|GetHas%20JustLanded) (Variables|Default|GetHasAttackOnce) (Variables|Default|GetHasAttackTwice) (Variables|Default|GetHasAttackThreeTimes)))
  (Sprite|SetFlipbook (Variables|Default|GetSprite) _output_flipbook))

(event Custom|ThirdAttack_Event_0
  (params (HasAttackedThreeTimes :type Boolean))
  (Development|PrintString "ThirdAttack")
  (Variables|Default|SetHasAttackThreeTimes true)
  (Utilities|FlowControl|Delay 1.0)
  (Variables|Default|SetHasAttackThreeTimes false))

(event Custom|FirstAttack_Event_0
  (params (HasAttackedOnce :type Boolean))
  (Variables|Default|SetHasAttackOnce true)
  (Utilities|FlowControl|Delay 0.5)
  (Variables|Default|SetHasAttackOnce false))

(event EventBeginPlay)

(event EventActorBeginOverlap
  (params (OtherActor :type Actor%20Object%20Reference)))

(event EventOnLanded
  (params (Hit :type Hit%20Result%20Structure%20%28by%20ref%29))
  (Variables|Default|SetHas%20JustLanded true)
  (Utilities|FlowControl|Delay 0.4)
  (Variables|Default|SetHas%20JustLanded false))

(event EventTick
  (params (DeltaSeconds :type Float%20%28single-precision%29))
  (Utilities|FlowControl|Sequence
    (:then_0
      (CallFunction|UpdateAnimation))
    (:then_1
      (if (Variables|Default|GetbIsDead)
        (Collision|SetCollisionEnabled (Variables|Default|GetCapsuleComponent) "NoCollision")
        (else
          (Collision|SetCollisionEnabled (Variables|Default|GetCapsuleComponent) "QueryAndPhysics"))))
    (:then_2
      (EventDispatchers|BindEventtoFirstAttack (delegate Custom|FirstAttack_Event_0))
      (EventDispatchers|AssignSecondAttack (delegate Custom|SecondAttack_Event_0))
      (EventDispatchers|AssignThirdAttack (delegate Custom|ThirdAttack_Event_0)))))

(fn ConstructionScript)

(fn AnimationStateMachine
  (params (is%20Falling :type Boolean) (is%20Moving :type Boolean) (Is%20Dead :type Boolean) (Has%20Just%20Landed :type Boolean) (HasAttackedOnce :type Boolean) (HasAttackedTwice :type Boolean) (HasAttackedThreeTimes :type Boolean))
  (LocalVariables|SetIsFallingLocal is%20Falling)
  (LocalVariables|SetIsMovingLocal is%20Moving)
  (LocalVariables|SetIsDeadLocal Is%20Dead)
  (LocalVariables|SetHasJustLandedLocal Has%20Just%20Landed)
  (LocalVariables|SetHasAttackedOnceLocal HasAttackedOnce)
  (LocalVariables|SetHasAttackedTwiceLocal HasAttackedTwice)
  (LocalVariables|SetHasAttackedThreeTimesLocal HasAttackedThreeTimes)
  (if (LocalVariables|GetHasAttackedThreeTimesLocal)
    (LocalVariables|SetAnimationState "NewEnumerator7")
    (elif (LocalVariables|GetHasAttackedTwiceLocal)
      (LocalVariables|SetAnimationState "NewEnumerator6")
      (elif (LocalVariables|GetHasAttackedOnceLocal)
        (LocalVariables|SetAnimationState "NewEnumerator5")
        (elif (LocalVariables|GetHasJustLandedLocal)
          (LocalVariables|SetAnimationState "NewEnumerator4")
          (elif (LocalVariables|GetIsDeadLocal)
            (LocalVariables|SetAnimationState "NewEnumerator3")
            (elif (LocalVariables|GetIsFallingLocal)
              (LocalVariables|SetAnimationState "NewEnumerator2")
              (elif (LocalVariables|GetIsMovingLocal)
                (LocalVariables|SetAnimationState "NewEnumerator1")
                (else
                  (LocalVariables|SetAnimationState "NewEnumerator0")))))))))
  (return (Utilities|Select :Index (LocalVariables|GetAnimationState) :NewEnumerator0 "/Game/FlipBooks/Dash_SwordMan/idle.idle" :NewEnumerator1 "/Game/FlipBooks/Dash_SwordMan/Running.Running" :NewEnumerator2 "/Game/FlipBooks/Dash_SwordMan/Jumping.Jumping" :NewEnumerator3 "/Game/2dSideScroller/Sprites/RunningAnimation.RunningAnimation" :NewEnumerator4 "/Game/FlipBooks/Dash_SwordMan/justlanded.justlanded" :NewEnumerator5 "/Game/FlipBooks/Dash_SwordMan/justlanded.justlanded" :NewEnumerator6 "/Game/2dSideScroller/Sprites/IdleAnimation.IdleAnimation" :NewEnumerator7 "/Game/FlipBooks/Dash_SwordMan/Jumping.Jumping")))